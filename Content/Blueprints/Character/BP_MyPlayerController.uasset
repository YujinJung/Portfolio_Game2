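; Player controller for a voxel game that handles the quick slot bar, inventory and pause UI, plus hand animation input.
; InitializeUMG creates the three widgets, with inventory and resume screens hidden; E and Escape call PauseGame and toggle them through one shared open flag.
; Number keys and mouse wheel change the quick slot, then update the character's held voxel.
; The left-click axis drives the character's hand location and rotation animations.
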(event Custom|Initialize%20UMG
  ;[1 1 1] Initialize UI
  (Utilities|FlowControl|Sequence
    (:then_0
      (bind _returnvalue (UserInterface|CreateWidget "/Game/Blueprints/UI/BP_UMG_QuickSlot.BP_UMG_QuickSlot_C"))
      (UserInterface|Viewport|AddtoViewport _returnvalue 0)
      (Variables|UI|SetQuickSlotWidget _returnvalue))
    (:then_1
      (bind _returnvalue_2 (UserInterface|CreateWidget "/Game/Blueprints/UI/BP_UMG_Inventory.BP_UMG_Inventory_C"))
      (UserInterface|Viewport|AddtoViewport _returnvalue_2 0)
      (bind _output_get (Variables|UI|SetInventoryWidget _returnvalue_2))
      (Widget|SetVisibility _output_get "Hidden")
      (Variables|Default|SetbCheckOpenInventory true))
    (:then_2
      (Variables|Default|SetbIsFlyItem (Variables|Default|GetbIsFlyItem)))
    (:then_3
      (bind _returnvalue_3 (UserInterface|CreateWidget "/Game/Blueprints/UI/BP_UMG_Resume.BP_UMG_Resume_C"))
      (UserInterface|Viewport|AddtoViewport _returnvalue_3 0)
      (bind _output_get_2 (Variables|UI|SetResumeWidget _returnvalue_3))
      (Widget|SetVisibility _output_get_2 "Hidden"))))

(event EventBeginPlay
  (bind _asbp_character (Utilities|Casting|CastToBP_Character (Game|Player|GetPlayerPawn 0)))
  (Variables|Player|SetPlayer_Ref _asbp_character))

(event EventTick
  (params (DeltaSeconds :type Float%20%28single-precision%29)))

(event Input|ActionEvents|InputActionLClick
  (params (Key :type Key%20Structure)))

(event Input|AxisEvents|InputAxisLClickScale
  (params (AxisValue :type Float%20%28single-precision%29))
  (bind _returnvalue (* AxisValue 2.0))
  (bind _player_ref (Variables|Player|GetPlayer_Ref))
  (Default|MoveHandLocationAnimation _player_ref _returnvalue)
  (Default|MoveHandRotationAnimation _player_ref _returnvalue))

(event Input|KeyboardEvents|5
  (params (Key :type Key%20Structure))
  ;[1 1 1] Quick Slot Widget Shortcut
  (:Pressed
    (Default|QuickSlotKeyboardEvent (Variables|UI|GetQuickSlotWidget) 4)
    (Default|ChangeVoxelinHand (Variables|Player|GetPlayer_Ref))))

(event Input|KeyboardEvents|1
  (params (Key :type Key%20Structure))
  ;[1 1 1] Quick Slot Widget Shortcut
  (:Pressed
    (Default|QuickSlotKeyboardEvent (Variables|UI|GetQuickSlotWidget))
    (Default|ChangeVoxelinHand (Variables|Player|GetPlayer_Ref))))

(event Input|MouseEvents|MouseWheelUp
  (params (Key :type Key%20Structure))
  ;[1 1 1] Quick Slot Widget Shortcut
  (:Pressed
    (Default|QuickSlotMouseWheelUp (Variables|UI|GetQuickSlotWidget))
    (Default|ChangeVoxelinHand (Variables|Player|GetPlayer_Ref))))

(event Input|KeyboardEvents|Escape
  (params (Key :type Key%20Structure))
  (bind _resumewidget (Variables|UI|GetResumeWidget))
  ;[1 1 1] Pause UI
  (:Pressed
    (Class|MyPlayerController|PauseGame)
    (if (Variables|Default|GetbCheckOpenInventory)
      (Widget|SetVisibility _resumewidget "Visible")
      (Variables|Default|SetbCheckOpenInventory false)
      (Class|MyPlayerController|SetIsOpenInventory true)
      (else
        (Widget|SetVisibility _resumewidget "Hidden")
        (Variables|Default|SetbCheckOpenInventory true)
        (Class|MyPlayerController|SetIsOpenInventory false)))))

(event Input|KeyboardEvents|E
  (params (Key :type Key%20Structure))
  ;[1 1 1] Open/Close Inventory
  (:Pressed
    (Class|MyPlayerController|PauseGame)
    (if (Variables|Default|GetbCheckOpenInventory)
      (Widget|SetVisibility (Variables|UI|GetInventoryWidget) "Visible")
      (Variables|Default|SetbCheckOpenInventory false)
      (Class|MyPlayerController|SetIsOpenInventory true)
      (else
        (Widget|SetVisibility (Variables|UI|GetInventoryWidget) "Hidden")
        (Variables|Default|SetbCheckOpenInventory true)
        (Class|MyPlayerController|SetIsOpenInventory false)))))

(event Input|KeyboardEvents|2
  (params (Key :type Key%20Structure))
  ;[1 1 1] Quick Slot Widget Shortcut
  (:Pressed
    (Default|QuickSlotKeyboardEvent (Variables|UI|GetQuickSlotWidget) 1)
    (Default|ChangeVoxelinHand (Variables|Player|GetPlayer_Ref))))

(event Input|KeyboardEvents|3
  (params (Key :type Key%20Structure))
  ;[1 1 1] Quick Slot Widget Shortcut
  (:Pressed
    (Default|QuickSlotKeyboardEvent (Variables|UI|GetQuickSlotWidget) 2)
    (Default|ChangeVoxelinHand (Variables|Player|GetPlayer_Ref))))

(event Input|KeyboardEvents|4
  (params (Key :type Key%20Structure))
  ;[1 1 1] Quick Slot Widget Shortcut
  (:Pressed
    (Default|QuickSlotKeyboardEvent (Variables|UI|GetQuickSlotWidget) 3)
    (Default|ChangeVoxelinHand (Variables|Player|GetPlayer_Ref))))

(event Input|KeyboardEvents|9
  (params (Key :type Key%20Structure))
  ;[1 1 1] Quick Slot Widget Shortcut
  (:Pressed
    (Default|QuickSlotKeyboardEvent (Variables|UI|GetQuickSlotWidget) 8)
    (Default|ChangeVoxelinHand (Variables|Player|GetPlayer_Ref))))

(event Input|KeyboardEvents|7
  (params (Key :type Key%20Structure))
  ;[1 1 1] Quick Slot Widget Shortcut
  (:Pressed
    (Default|QuickSlotKeyboardEvent (Variables|UI|GetQuickSlotWidget) 6)
    (Default|ChangeVoxelinHand (Variables|Player|GetPlayer_Ref))))

(event Input|KeyboardEvents|8
  (params (Key :type Key%20Structure))
  ;[1 1 1] Quick Slot Widget Shortcut
  (:Pressed
    (Default|QuickSlotKeyboardEvent (Variables|UI|GetQuickSlotWidget) 7)
    (Default|ChangeVoxelinHand (Variables|Player|GetPlayer_Ref))))

(event Input|KeyboardEvents|6
  (params (Key :type Key%20Structure))
  ;[1 1 1] Quick Slot Widget Shortcut
  (:Pressed
    (Default|QuickSlotKeyboardEvent (Variables|UI|GetQuickSlotWidget) 5)
    (Default|ChangeVoxelinHand (Variables|Player|GetPlayer_Ref))))

(event Input|MouseEvents|MouseWheelDown
  (params (Key :type Key%20Structure))
  ;[1 1 1] Quick Slot Widget Shortcut
  (:Pressed
    (Default|QuickSlotMouseWheelDown (Variables|UI|GetQuickSlotWidget))
    (Default|ChangeVoxelinHand (Variables|Player|GetPlayer_Ref))))

(fn ConstructionScript)