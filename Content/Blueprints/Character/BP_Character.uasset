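; BP_Character is a character Blueprint that owns the player's quick slot and inventory UI.
; On BeginPlay it creates both widgets, adds them to the viewport with the inventory hidden, and clears IsFlyItem.
; Number keys 1-9 and the mouse wheel forward selection events to the quick slot widget.
; E calls PauseGame and toggles inventory visibility through IsOpenInventory, which is inverted: true means hidden.
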(event EventBeginPlay
  (Utilities|FlowControl|Sequence
    (:then_1
      (bind _returnvalue (UserInterface|CreateWidget "/Game/Blueprints/UI/BP_UMG_QuickSlot.BP_UMG_QuickSlot_C"))
      (UserInterface|Viewport|AddtoViewport _returnvalue 0)
      (Variables|Widget|SetQuickSlotWidget _returnvalue))
    (:then_2
      (bind _returnvalue_2 (UserInterface|CreateWidget "/Game/Blueprints/UI/BP_UMG_Inventory.BP_UMG_Inventory_C"))
      (UserInterface|Viewport|AddtoViewport _returnvalue_2 0)
      (bind _output_get (Variables|Widget|SetInventoryWidget _returnvalue_2))
      (Widget|SetVisibility _output_get "Hidden")
      (Variables|Widget|SetisOpenInventory true))
    (:then_3
      (Variables|Item|SetisFlyItem false))))

(event Collision|EventActorBeginOverlap
  (params (OtherActor :type Actor%20Object%20Reference)))

(event EventTick
  (params (DeltaSeconds :type Float%20%28single-precision%29)))

(event Input|KeyboardEvents|5
  (params (Key :type Key%20Structure))
  ;[1 1 1] Quick Slot Widget Shortcut
  (:Pressed
    (Default|QuickSlotKeyboardEvent (Variables|Widget|GetQuickSlotWidget) 4)))

(event Input|KeyboardEvents|1
  (params (Key :type Key%20Structure))
  ;[1 1 1] Quick Slot Widget Shortcut
  (:Pressed
    (Default|QuickSlotKeyboardEvent (Variables|Widget|GetQuickSlotWidget))))

(event Input|MouseEvents|MouseWheelUp
  (params (Key :type Key%20Structure))
  ;[1 1 1] Quick Slot Widget Shortcut
  (:Pressed
    (Default|QuickSlotMouseWheelUp (Variables|Widget|GetQuickSlotWidget))))

(event Input|KeyboardEvents|E
  (params (Key :type Key%20Structure))
  (bind _inventorywidget (Variables|Widget|GetInventoryWidget))
  ;[1 1 1] Open/Close Inventory
  (:Pressed
    (Class|MyCharacter|PauseGame)
    (if (Variables|Widget|GetisOpenInventory)
      (Widget|SetVisibility _inventorywidget "Visible")
      (Variables|Widget|SetisOpenInventory false)
      (else
        (Widget|SetVisibility _inventorywidget "Hidden")
        (Variables|Widget|SetisOpenInventory true)))))

(event Input|KeyboardEvents|2
  (params (Key :type Key%20Structure))
  ;[1 1 1] Quick Slot Widget Shortcut
  (:Pressed
    (Default|QuickSlotKeyboardEvent (Variables|Widget|GetQuickSlotWidget) 1)))

(event Input|KeyboardEvents|3
  (params (Key :type Key%20Structure))
  ;[1 1 1] Quick Slot Widget Shortcut
  (:Pressed
    (Default|QuickSlotKeyboardEvent (Variables|Widget|GetQuickSlotWidget) 2)))

(event Input|KeyboardEvents|4
  (params (Key :type Key%20Structure))
  ;[1 1 1] Quick Slot Widget Shortcut
  (:Pressed
    (Default|QuickSlotKeyboardEvent (Variables|Widget|GetQuickSlotWidget) 3)))

(event Input|KeyboardEvents|9
  (params (Key :type Key%20Structure))
  ;[1 1 1] Quick Slot Widget Shortcut
  (:Pressed
    (Default|QuickSlotKeyboardEvent (Variables|Widget|GetQuickSlotWidget) 8)))

(event Input|KeyboardEvents|7
  (params (Key :type Key%20Structure))
  ;[1 1 1] Quick Slot Widget Shortcut
  (:Pressed
    (Default|QuickSlotKeyboardEvent (Variables|Widget|GetQuickSlotWidget) 6)))

(event Input|KeyboardEvents|8
  (params (Key :type Key%20Structure))
  ;[1 1 1] Quick Slot Widget Shortcut
  (:Pressed
    (Default|QuickSlotKeyboardEvent (Variables|Widget|GetQuickSlotWidget) 7)))

(event Input|KeyboardEvents|6
  (params (Key :type Key%20Structure))
  ;[1 1 1] Quick Slot Widget Shortcut
  (:Pressed
    (Default|QuickSlotKeyboardEvent (Variables|Widget|GetQuickSlotWidget) 5)))

(event Input|MouseEvents|MouseWheelDown
  (params (Key :type Key%20Structure))
  ;[1 1 1] Quick Slot Widget Shortcut
  (:Pressed
    (Default|QuickSlotMouseWheelDown (Variables|Widget|GetQuickSlotWidget))))

(fn ConstructionScript)